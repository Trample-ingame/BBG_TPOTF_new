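; Game instance that persists player settings for audio, graphics, content toggles and difficulty in the BBG_settings save slot.
; On Init it calls Loadgame if the slot exists, otherwise writes defaults, then loads GameUserSettings and sets GAMELAUNCHED after a two-second delay.
; Savegame writes every setting into a fresh Save_object, replacing the slot.
; Loadgame only returns the stored values; Init does not use them.
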(event EventInit
  (bind _returnvalue (SaveGame|DoesSaveGameExist "BBG_settings"))
  (if _returnvalue
    (CallFunction|Loadgame)
    (else
      (CallFunction|Savegame true 1.0 true 1.0 true 1.0 true 1.0 true true true true 0.5 "Fullscreen" "1920X1080" true true true false "NORMAL" false false false false)))
  (bind _returnvalue_2 (Settings|GetGameUserSettings))
  (Class|GameUserSettings|LoadSettings _returnvalue_2 true)
  (Utilities|FlowControl|Delay 2.0)
  (Variables|Default|SetGAME_LAUNCHED true))

(fn Savegame
  (params (MUSIC :type Boolean) (MUSIC_VOLUME :type Float%20%28single-precision%29) (AMBIENT :type Boolean) (AMBIENT_VOLUME :type Float%20%28single-precision%29) (VOICE :type Boolean) (VOICE_VOLUME :type Float%20%28single-precision%29) (FX :type Boolean) (FX_VOLUME :type Float%20%28single-precision%29) (VIBRATION :type Boolean) (HDOBJECTS :type Boolean) (MIST :type Boolean) (HIT_PRINTS :type Boolean) (HIT_PRINTS_TRANSPARENCY :type Float%20%28single-precision%29) (FULL_SCREEN :type EWindowMode%20Enum :default "Fullscreen") (RESOLUTION :type String) (FEET :type Boolean) (BUTT :type Boolean) (VORE :type Boolean) (NSFW :type Boolean) (DIFFICULTY :type String) (RAYTRACING :type Boolean) (DOF :type Boolean) (FUR :type Boolean) (foliage :type Boolean))
  (bind _returnvalue (SaveGame|CreateSaveGameObject "/Game/Blueprints/save_object.save_object_C"))
  (bind _output_get (Variables|Default|Setsave_ref _returnvalue))
  (Utilities|FlowControl|Sequence
    (:then_0
      (Variables|/Game/Blueprints/save_object.save_object_C|SetMUSIC _output_get MUSIC)
      (Variables|/Game/Blueprints/save_object.save_object_C|SetAMBIENT _output_get AMBIENT)
      (Variables|/Game/Blueprints/save_object.save_object_C|SetVOICE _output_get VOICE)
      (Variables|/Game/Blueprints/save_object.save_object_C|SetFX _output_get FX))
    (:then_1
      (Variables|/Game/Blueprints/save_object.save_object_C|SetMUSIC_VOLUME _output_get MUSIC_VOLUME)
      (Variables|/Game/Blueprints/save_object.save_object_C|SetAMBIENT_VOLUME _output_get AMBIENT_VOLUME)
      (Variables|/Game/Blueprints/save_object.save_object_C|SetVOICE_VOLUME _output_get VOICE_VOLUME)
      (Variables|/Game/Blueprints/save_object.save_object_C|SetFX_VOLUME _output_get FX_VOLUME))
    (:then_2
      (Variables|/Game/Blueprints/save_object.save_object_C|SetFUR _output_get FUR)
      (Variables|/Game/Blueprints/save_object.save_object_C|SetHDOBJECTS _output_get HDOBJECTS)
      (Variables|/Game/Blueprints/save_object.save_object_C|SetMIST _output_get MIST)
      (Variables|/Game/Blueprints/save_object.save_object_C|SetHIT_PRINTS _output_get HIT_PRINTS)
      (Variables|/Game/Blueprints/save_object.save_object_C|SetHIT_PRINTS_TRANSPARENCY _output_get HIT_PRINTS_TRANSPARENCY))
    (:then_3
      (Variables|/Game/Blueprints/save_object.save_object_C|SetFULL_SCREEN _output_get FULL_SCREEN)
      (Variables|/Game/Blueprints/save_object.save_object_C|SetRESOLUTION _output_get RESOLUTION)
      (Variables|/Game/Blueprints/save_object.save_object_C|SetRAYTRACING _output_get RAYTRACING)
      (Variables|/Game/Blueprints/save_object.save_object_C|SetDOF _output_get DOF))
    (:then_4
      (Variables|/Game/Blueprints/save_object.save_object_C|SetFEET _output_get FEET)
      (Variables|/Game/Blueprints/save_object.save_object_C|SetBUTT _output_get BUTT)
      (Variables|/Game/Blueprints/save_object.save_object_C|SetVORE _output_get VORE)
      (Variables|/Game/Blueprints/save_object.save_object_C|SetNSFW _output_get NSFW))
    (:then_5
      (Variables|/Game/Blueprints/save_object.save_object_C|SetDIFFICULTY _output_get DIFFICULTY)
      (Variables|/Game/Blueprints/save_object.save_object_C|SetVIBRATION _output_get VIBRATION)
      (Variables|/Game/Blueprints/save_object.save_object_C|Setfoliage _output_get foliage)
      (SaveGame|SaveGametoSlot _output_get "BBG_settings"))))

(fn Loadgame
  (bind _returnvalue (SaveGame|DoesSaveGameExist "BBG_settings"))
  (if _returnvalue
    (bind _returnvalue_2 (SaveGame|LoadGamefromSlot "BBG_settings"))
    (bind _assave_object (Utilities|Casting|CastTosave_object _returnvalue_2))
    (return (Variables|/Game/Blueprints/save_object.save_object_C|GetMUSIC _assave_object) (Variables|/Game/Blueprints/save_object.save_object_C|GetMUSIC_VOLUME _assave_object) (Variables|/Game/Blueprints/save_object.save_object_C|GetAMBIENT _assave_object) (Variables|/Game/Blueprints/save_object.save_object_C|GetAMBIENT_VOLUME _assave_object) (Variables|/Game/Blueprints/save_object.save_object_C|GetVOICE _assave_object) (Variables|/Game/Blueprints/save_object.save_object_C|GetVOICE_VOLUME _assave_object) (Variables|/Game/Blueprints/save_object.save_object_C|GetFX _assave_object) (Variables|/Game/Blueprints/save_object.save_object_C|GetFX_VOLUME _assave_object) (Variables|/Game/Blueprints/save_object.save_object_C|GetVIBRATION _assave_object) (Variables|/Game/Blueprints/save_object.save_object_C|GetHDOBJECTS _assave_object) (Variables|/Game/Blueprints/save_object.save_object_C|GetMIST _assave_object) (Variables|/Game/Blueprints/save_object.save_object_C|GetHIT_PRINTS _assave_object) (Variables|/Game/Blueprints/save_object.save_object_C|GetHIT_PRINTS_TRANSPARENCY _assave_object) (Variables|/Game/Blueprints/save_object.save_object_C|GetFULL_SCREEN _assave_object) (Variables|/Game/Blueprints/save_object.save_object_C|GetRESOLUTION _assave_object) (Variables|/Game/Blueprints/save_object.save_object_C|GetFEET _assave_object) (Variables|/Game/Blueprints/save_object.save_object_C|GetBUTT _assave_object) (Variables|/Game/Blueprints/save_object.save_object_C|GetVORE _assave_object) (Variables|/Game/Blueprints/save_object.save_object_C|GetNSFW _assave_object) (Variables|/Game/Blueprints/save_object.save_object_C|GetDIFFICULTY _assave_object) (Variables|/Game/Blueprints/save_object.save_object_C|GetRAYTRACING _assave_object) (Variables|/Game/Blueprints/save_object.save_object_C|GetDOF _assave_object) (Variables|/Game/Blueprints/save_object.save_object_C|GetFUR _assave_object) (Variables|/Game/Blueprints/save_object.save_object_C|Getfoliage _assave_object))))